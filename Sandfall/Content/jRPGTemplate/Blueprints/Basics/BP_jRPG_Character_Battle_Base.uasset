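; Co-op mod hooks for the base jRPG battle character that assign party members to local players by battle spot.
; Turn start announces the player and hands controller 0 to that player's platform user; turn end restores the primary user.
; Parry, gradient parry, dodge, jump and jump counter reach their orig_ functions only for player 1's or non-player characters.
; Defensive moves scale the immunity window by per-player co-op config.
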(fn ConstructionScript)

(fn HookTryStartParry
  (Utilities|IsCharacterControlledbyPlayer1
    (:then
      (bind _success (CallFunction|OrigTryStartParry))
      (return _success))
    (:else
      (return false))))

(fn OrigTryStartParry
  (return false))

(fn HookonTurnStart
  (bind _returnvalue (Game|GetPlayerController 0))
  (Utilities|FlowControl|Sequence
    (:then_0
      (if (Variables|Default|GetIsPlayerControlledCharacter)
        (bind (_user _index) (CallFunction|MapBattleSpottoUser (Variables|Default|GetBattleSpotIndex)))
        (bind _asbp_j_rpg_controller_world (Utilities|Casting|CastToBP_jRPG_Controller_World _returnvalue))
        (Default|ShowBattleTooltip (Variables|/Game/jRPGTemplate/Blueprints/Basics/BP_jRPG_Controller_World.BP_jRPG_Controller_World_C|GetAC_jRPG_BattleManager _asbp_j_rpg_controller_world) (Utilities|Text|FormatText "Player {i}'s Turn" (+ _index 1)) true)
        (Class|GameplayStatics|SetPlayerPlatformUserId _returnvalue (Class|InputDeviceLibrary|GetPrimaryPlatformUser)) ; First revert to primary platform user, in case someone took over temporarily
        (Class|GameplayStatics|SetPlayerPlatformUserId _returnvalue _user)))
    (:then_1
      (CallFunction|OrigonTurnStart))))

(fn OrigonTurnStart)

(fn HookonTurnEnded
  (CallFunction|OrigonTurnEnded)
  (if (Variables|Default|GetIsPlayerControlledCharacter)
    (Class|GameplayStatics|SetPlayerPlatformUserId (Game|GetPlayerController 0) (Class|InputDeviceLibrary|GetPrimaryPlatformUser))))

(fn OrigonTurnEnded)

(fn HookTryStartDodge
  (Utilities|IsCharacterControlledbyPlayer1
    (:then
      (bind _success (CallFunction|OrigTryStartDodge))
      (return _success))
    (:else
      (return false))))

(fn OrigTryStartDodge
  (return false))

(fn HookTryTriggerJumpCounterAttack
  (Utilities|IsCharacterControlledbyPlayer1
    (:then
      (CallFunction|OrigTryTriggerJumpCounterAttack)
      (return))
    (:else
      (return))))

(fn OrigTryTriggerJumpCounterAttack)

(fn HookTryStartJump
  (Utilities|IsCharacterControlledbyPlayer1
    (:then
      (bind _success (CallFunction|OrigTryStartJump))
      (return _success))
    (:else
      (return false))))

(fn OrigTryStartJump
  (return false))

(fn HookTryStartGradientParry
  (Utilities|IsCharacterControlledbyPlayer1
    (:then
      (bind _success (CallFunction|OrigTryStartGradientParry))
      (return _success))
    (:else
      (return false))))

(fn OrigTryStartGradientParry
  (return false))

(fn HookStartDefensiveMove
  (params (LockDuration :type Float%20%28double-precision%29) (ImmuneDuration :type Float%20%28double-precision%29) (WarmUpDuration :type Float%20%28double-precision%29) (Reason :type String))
  (bind _coop_config (CallFunction|LoadCoopConfig))
  (bind _index (CallFunction|MapBattleSpottoUser (Variables|Default|GetBattleSpotIndex)))
  (CallFunction|OrigStartDefensiveMove LockDuration (* ImmuneDuration (Default|GetPlayerDefenseWindow _coop_config _index)) WarmUpDuration Reason))

(fn OrigStartDefensiveMove
  (params (LockDuration :type Float%20%28double-precision%29) (ImmuneDuration :type Float%20%28double-precision%29) (WarmUpDuration :type Float%20%28double-precision%29) (Reason :type String)))