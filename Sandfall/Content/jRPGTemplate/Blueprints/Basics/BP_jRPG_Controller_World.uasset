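; World (exploration) controller for the jRPG template, which reports that it is never in battle and hooks map changes and battle end.
; Before a map change it removes every extra local player and pawn, then reassigns the first controller to the primary platform user.
; When exploration resumes after battle it makes the same reassignment.
; Both hook_ functions then call their empty orig_ counterparts, a wrapper pattern around the original logic.
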(event EventBeginPlay)

(event EventTick
  (params (DeltaSeconds :type Float%20%28single-precision%29)))

(fn ConstructionScript)

(fn IsinBattle
  (return false))

(fn HookPreparetoChangeMap
  (params (LevelData :type F%20Level%20Data%20Entry%20Structure%20%28by%20ref%29))
  (while (> (Class|GameplayStatics|GetNumPlayerControllers) 1)
    (Class|GameplayStatics|RemovePlayer (Game|GetPlayerController 1) true))
  (Class|GameplayStatics|SetPlayerPlatformUserId (Game|GetPlayerController 0) (Class|InputDeviceLibrary|GetPrimaryPlatformUser))
  (CallFunction|OrigPreparetoChangeMap LevelData))

(fn OrigPreparetoChangeMap
  (params (LevelData :type F%20Level%20Data%20Entry%20Structure%20%28by%20ref%29)))

(fn HookResumeExplorationonBattleEnd
  (params (EnemyGlobalID :type Name) (BattleEndResult :type EBattleEndResult%20Enum :default "NewEnumerator0"))
  (Class|GameplayStatics|SetPlayerPlatformUserId (Game|GetPlayerController 0) (Class|InputDeviceLibrary|GetPrimaryPlatformUser))
  (CallFunction|OrigResumeExplorationonBattleEnd EnemyGlobalID BattleEndResult))

(fn OrigResumeExplorationonBattleEnd
  (params (EnemyGlobalID :type Name) (BattleEndResult :type EBattleEndResult%20Enum :default "NewEnumerator0")))